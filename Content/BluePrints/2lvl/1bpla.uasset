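; Actor Blueprint in a 2lvl folder that blinks a point light a set number of times when play begins.
; If IsTrue is set, BeginPlay runs a counted loop through a Delay of Speed seconds until Cnt reaches twice Nb.
; Each pass flips the light's visibility on or off through a FlipFlop, giving Nb blinks, and prints a string to screen.
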(event `self.ReceiveBeginPlay`
  (bind _cnt (`self.cnt`))
  (bind _pointlight (`self.PointLight`))
  (if (`self.isTrue`)
    (if (< _cnt (* (`self.nb`) 2)) :!label _label
      (set `self.cnt` (+ _cnt 1))
      (`KismetSystemLibrary.Delay` (`self.speed`))
      (`/Engine/EditorBlueprintResources/StandardMacros.FlipFlop`
        (:`A`
          (`SceneComponent.SetVisibility` _pointlight true false))
        (:`B`
          (`SceneComponent.SetVisibility` _pointlight false false)))
      (`KismetSystemLibrary.PrintString` "Hello" true true (struct :`G` 0.66 :`B` 1.0 :`A` 1.0) 3.0)
      (goto _label))))

(fn `UserConstructionScript`)