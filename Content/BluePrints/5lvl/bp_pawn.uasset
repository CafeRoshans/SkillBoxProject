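; Player pawn for level 5 that slides sideways along Y and spawns a Sharik actor at its capsule on BeginPlay.
; MoveRight input steps the pawn a fixed offset left or right, gated by free-side flags; each move's InitialOverlap result sets the opposite side's flag.
; Tick clamps Y within symmetric limits.
; SpawnSharik stores the spawned actor and binds a handler to its ONDEAD event.
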(event `InputAxis|MoveRight`
  (params (AxisValue :type "Float (single-precision)"))
  (if (< AxisValue 0.0)
    (if (`self.LeftIsFree`)
      (bind _sweephitresult (`self.K2_AddActorWorldTransform` (`KismetMathLibrary.MakeTransform` (0.0 -50.0 0.0))))
      (if (`.bInitialOverlap` (`GameplayStatics.BreakHitResult` _sweephitresult))
        (set `self.RightIsFree` false)
        (else
          (set `self.RightIsFree` true))))))

(event `InputAxis|MoveRight`
  (params (AxisValue :type "Float (single-precision)"))
  (if (> AxisValue 0.0)
    (if (`self.RightIsFree`)
      (bind _sweephitresult (`self.K2_AddActorWorldTransform` (`KismetMathLibrary.MakeTransform` (0.0 50.0 0.0))))
      (if (`.bInitialOverlap` (`GameplayStatics.BreakHitResult` _sweephitresult))
        (set `self.LeftIsFree` false)
        (else
          (set `self.LeftIsFree` true))))))

(event `self.ReceiveBeginPlay`
  (`self.spawnSharik`))

(event `self.ReceiveTick`
  (params (DeltaSeconds :type "Float (single-precision)"))
  (bind _x (.x (`self.K2_GetActorLocation`)))
  (bind _y (.y (`self.K2_GetActorLocation`)))
  (bind _z (.z (`self.K2_GetActorLocation`)))
  (if (> _y 1000.0)
    (`self.K2_SetActorLocation` (`KismetMathLibrary.MakeVector` _x 1000.0 _z))
    (elif (< _y -1000.0)
      (`self.K2_SetActorLocation` (`KismetMathLibrary.MakeVector` _x -1000.0 _z)))))

(fn `spawnSharik`
  (bind _returnvalue (`|SpawnActorFromClass` "/Game/BluePrints/3lvl/Sharik.Sharik_C" (`SceneComponent.K2_GetComponentToWorld` (`self.Capsule`)) "AlwaysSpawn" "OverrideRootScale" null null))
  (bind _output_get (set `self.NewSharik` _returnvalue))
  (add `/Game/BluePrints/3lvl/Sharik.ONDEAD` _output_get (`|CreateDelegate` :!event `spawnSharik`))
  (return))

(fn `UserConstructionScript`)